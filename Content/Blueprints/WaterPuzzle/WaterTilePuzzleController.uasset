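; Controller for a water tile puzzle, apparently unfinished: its events are empty and neither function is called within it.
; CheckTiles finds the SourceTile and gathers TileBP actors, excluding source and end tiles by display name, then enters an empty loop on BreakLoop.
; WaterTileCheck fills a 25-slot boolean water array and flags the first slot when the source overlaps a WaterCheck-tagged component, with no action on the result.
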(fn `CheckTiles`
  (bind _returnvalue (`GameplayStatics.GetActorOfClass` "/Game/Blueprints/WaterPuzzle/SourceTile.SourceTile_C"))
  (set `self.SourceTile` _returnvalue)
  (bind _outactors (`GameplayStatics.GetAllActorsOfClass` "/Game/Blueprints/WaterPuzzle/TileBP.TileBP_C"))
  (for _array_element _outactors
    (bind _returnvalue_2 (`KismetSystemLibrary.GetDisplayName` _array_element))
    (if (not (or (`KismetStringLibrary.EqualEqual_StrStr` _returnvalue_2 "SourceTile") (`KismetStringLibrary.EqualEqual_StrStr` _returnvalue_2 "EndTile")))
      (`KismetArrayLibrary.Array_Add` (`self.TileArray`) _array_element)))
  (while (`self.BreakLoop?`)
    _))

(fn `UserConstructionScript`)

(fn `WaterTileCheck`
  (bind _waterarray (`self.WaterArray`))
  (for _ (range 1 26)
    (`KismetArrayLibrary.Array_Add` (`self.WaterArray`)))
  (bind _returnvalue (`GameplayStatics.GetActorOfClass` "/Game/Blueprints/WaterPuzzle/SourceTile.SourceTile_C"))
  (set `self.SourceTile` _returnvalue)
  (for _array_element (`self.GetOverlappingComponents` (`self.SourceTile`))
    (if (`ActorComponent.ComponentHasTag` _array_element "WaterCheck")
      (`KismetArrayLibrary.Array_Set` _waterarray 0 true)))
  (if (`|GetArrayItem` _waterarray)
    _))