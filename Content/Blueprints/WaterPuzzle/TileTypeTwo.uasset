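; Water puzzle tile variant that decides whether it carries water from its neighbours.
; On BeginPlay and in CheckChannels, it tests four WaterCheck components in turn, stopping once the tile has water.
; Each check finds an overlapping WaterCheck-tagged component and looks for a HasWater tag on its parents.
; The result sets the tile's HasWater tag and on/off material, with debug prints throughout.
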(event `self.ReceiveBeginPlay`
  (`parent.ReceiveBeginPlay`)
  (`self.CheckChannels`))

(fn `CheckChannels`
  (`parent.CheckChannels`)
  ;[1 1 1] WaterCheck1
  (`KismetSystemLibrary.PrintString` "in check channels")
  (for _array_element (`PrimitiveComponent.GetOverlappingComponents` (`self.WaterCheck1`))
    (if (`ActorComponent.ComponentHasTag` _array_element "WaterCheck")
      (`KismetSystemLibrary.PrintString` "has water check tag" true true (struct :`G` 0.66 :`B` 1.0 :`A` 1.0) 15.0)
      (for _array_element_2 (`SceneComponent.GetParentComponents` _array_element)
        (if (`ActorComponent.ComponentHasTag` _array_element_2 "HasWater")
          (`KismetSystemLibrary.PrintString` "overlapped has water" true true (struct :`G` 0.66 :`B` 1.0 :`A` 1.0) 15.0)
          (`PrimitiveComponent.SetMaterial` (`self.Tile`) 0 "/Game/Materials/WaterTileTempOn.WaterTileTempOn")
          (set `ActorComponent.ComponentTags` (`|MakeArray` "HasWater" :!type "Name") (`self.Tile`)) ; Tile (self) has water
          (break)
          (else
            (`KismetSystemLibrary.PrintString` "overlapped does not haswater" true true (struct :`G` 0.66 :`B` 1.0 :`A` 1.0) 15.0)
            (set `ActorComponent.ComponentTags` (`|MakeArray` "None" :!type "Name") (`self.Tile`)) ; Tile (self) has no water
            (`PrimitiveComponent.SetMaterial` (`self.Tile`) 0 "/Game/Materials/WaterTileTempOff.WaterTileTempOff"))))
      (break)
      (else
        (`KismetSystemLibrary.PrintString` "does not have water check tag" true true (struct :`G` 0.66 :`B` 1.0 :`A` 1.0) 15.0))))
  (if (not (`ActorComponent.ComponentHasTag` (`self.Tile`) "HasWater"))
    ;[1 1 1] WaterCheck2
    (`KismetSystemLibrary.PrintString` "in check channels")
    (for _array_element_3 (`PrimitiveComponent.GetOverlappingComponents` (`self.WaterCheck2`))
      (if (`ActorComponent.ComponentHasTag` _array_element_3 "WaterCheck")
        (`KismetSystemLibrary.PrintString` "has water check tag" true true (struct :`G` 0.66 :`B` 1.0 :`A` 1.0) 15.0)
        (for _array_element_4 (`SceneComponent.GetParentComponents` _array_element_3)
          (if (`ActorComponent.ComponentHasTag` _array_element_4 "HasWater")
            (`KismetSystemLibrary.PrintString` "overlapped has water" true true (struct :`G` 0.66 :`B` 1.0 :`A` 1.0) 15.0)
            (`PrimitiveComponent.SetMaterial` (`self.Tile`) 0 "/Game/Materials/WaterTileTempOn.WaterTileTempOn")
            (set `ActorComponent.ComponentTags` (`|MakeArray` "HasWater" :!type "Name") (`self.Tile`)) ; Tile (self) has water
            (break)
            (else
              (`KismetSystemLibrary.PrintString` "overlapped does not haswater" true true (struct :`G` 0.66 :`B` 1.0 :`A` 1.0) 15.0)
              (set `ActorComponent.ComponentTags` (`|MakeArray` "None" :!type "Name") (`self.Tile`)) ; Tile (self) has no water
              (`PrimitiveComponent.SetMaterial` (`self.Tile`) 0 "/Game/Materials/WaterTileTempOff.WaterTileTempOff"))))
        (break)
        (else
          (`KismetSystemLibrary.PrintString` "does not have water check tag" true true (struct :`G` 0.66 :`B` 1.0 :`A` 1.0) 15.0))))
    (if (not (`ActorComponent.ComponentHasTag` (`self.Tile`) "HasWater"))
      ;[1 1 1] WaterCheck3
      (`KismetSystemLibrary.PrintString` "in check channels")
      (for _array_element_5 (`PrimitiveComponent.GetOverlappingComponents` (`self.WaterCheck3`))
        (if (`ActorComponent.ComponentHasTag` _array_element_5 "WaterCheck")
          (`KismetSystemLibrary.PrintString` "has water check tag" true true (struct :`G` 0.66 :`B` 1.0 :`A` 1.0) 15.0)
          (for _array_element_6 (`SceneComponent.GetParentComponents` _array_element_5)
            (if (`ActorComponent.ComponentHasTag` _array_element_6 "HasWater")
              (`KismetSystemLibrary.PrintString` "overlapped has water" true true (struct :`G` 0.66 :`B` 1.0 :`A` 1.0) 15.0)
              (`PrimitiveComponent.SetMaterial` (`self.Tile`) 0 "/Game/Materials/WaterTileTempOn.WaterTileTempOn")
              (set `ActorComponent.ComponentTags` (`|MakeArray` "HasWater" :!type "Name") (`self.Tile`)) ; Tile (self) has water
              (break)
              (else
                (`KismetSystemLibrary.PrintString` "overlapped does not haswater" true true (struct :`G` 0.66 :`B` 1.0 :`A` 1.0) 15.0)
                (set `ActorComponent.ComponentTags` (`|MakeArray` "None" :!type "Name") (`self.Tile`)) ; Tile (self) has no water
                (`PrimitiveComponent.SetMaterial` (`self.Tile`) 0 "/Game/Materials/WaterTileTempOff.WaterTileTempOff"))))
          (break)
          (else
            (`KismetSystemLibrary.PrintString` "does not have water check tag" true true (struct :`G` 0.66 :`B` 1.0 :`A` 1.0) 15.0))))
      (if (not (`ActorComponent.ComponentHasTag` (`self.Tile`) "HasWater"))
        ;[1 1 1] WaterCheck4
        (`KismetSystemLibrary.PrintString` "in check channels")
        (for _array_element_7 (`PrimitiveComponent.GetOverlappingComponents` (`self.WaterCheck4`))
          (if (`ActorComponent.ComponentHasTag` _array_element_7 "WaterCheck")
            (`KismetSystemLibrary.PrintString` "has water check tag" true true (struct :`G` 0.66 :`B` 1.0 :`A` 1.0) 15.0)
            (for _array_element_8 (`SceneComponent.GetParentComponents` _array_element_7)
              (if (`ActorComponent.ComponentHasTag` _array_element_8 "HasWater")
                (`KismetSystemLibrary.PrintString` "overlapped has water" true true (struct :`G` 0.66 :`B` 1.0 :`A` 1.0) 15.0)
                (`PrimitiveComponent.SetMaterial` (`self.Tile`) 0 "/Game/Materials/WaterTileTempOn.WaterTileTempOn")
                (set `ActorComponent.ComponentTags` (`|MakeArray` "HasWater" :!type "Name") (`self.Tile`)) ; Tile (self) has water
                (break)
                (else
                  (`KismetSystemLibrary.PrintString` "overlapped does not haswater" true true (struct :`G` 0.66 :`B` 1.0 :`A` 1.0) 15.0)
                  (set `ActorComponent.ComponentTags` (`|MakeArray` "None" :!type "Name") (`self.Tile`)) ; Tile (self) has no water
                  (`PrimitiveComponent.SetMaterial` (`self.Tile`) 0 "/Game/Materials/WaterTileTempOff.WaterTileTempOff"))))
            (break)
            (else
              (`KismetSystemLibrary.PrintString` "does not have water check tag" true true (struct :`G` 0.66 :`B` 1.0 :`A` 1.0) 15.0))))
        (if (`ActorComponent.ComponentHasTag` (`self.Tile`) "HasWater")
          _)))))

(fn `UserConstructionScript`
  (`parent.UserConstructionScript`))