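; BoxMirror is an interactable box actor that gives the player the mirror item once.
; On Interactable, it finds the MainCharacter, shows the found-object notice on its inventory widget and adds the mirror's image and hash code from InventoryStruct.
; It then sets its GotMirror flag to block repeat pickups and sets HaveMirror on the character.
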(event `self.ReceiveBeginPlay`)

(event `/Game/Blueprints/iInteract.Interactable`
  (bind (_inventorystruct_key _inventorystruct_statuette _inventorystruct_mirror) (break `/Game/Blueprints/InventoryStruct` (`self.InventoryStruct`)))
  (bind (_inventorystruct_key_2 _inventorystruct_statuette_2 _inventorystruct_mirror_2 _inventorystruct_mirrorhc) (break `/Game/Blueprints/InventoryStruct` (`self.InventoryStruct`)))
  (if (not (`self.gotMirror?`))
    (bind _returnvalue (`GameplayStatics.GetActorOfClass` "/Game/Blueprints/MainCharacter.MainCharacter_C"))
    (bind _inventorywidget (`/Game/Blueprints/MainCharacter.InventoryWidget` _returnvalue))
    (`/Game/UI/InventoryWidget.FoundObject` _inventorywidget _inventorystruct_mirror)
    (`/Game/UI/InventoryWidget.AddItemToInv` _inventorywidget _inventorystruct_mirror_2 _inventorystruct_mirrorhc)
    (set `self.gotMirror?` true)
    (bind _returnvalue_2 (`GameplayStatics.GetActorOfClass` "/Game/Blueprints/MainCharacter.MainCharacter_C"))
    (set `/Game/Blueprints/MainCharacter.HaveMirror?` true _returnvalue_2)))

(fn `UserConstructionScript`)