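; First-person-style player character that handles movement, look, object interaction and an inventory UI.
; Each tick a debug-drawn camera line trace tracks the last hit IInteract actor, sending it NonInteractableMessage while no interactable is hit.
; Interact sends InteractableMessage to that actor when the trace is on an interactable.
; An inventory widget created at BeginPlay receives Pickup presses and items passed through AddItemMC with a hash code.
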(event `self.ReceiveBeginPlay`
  (bind _returnvalue (`|CreateWidget` "/Game/UI/InventoryWidget.InventoryWidget_C"))
  (bind _output_get (set `self.InventoryWidget` _returnvalue))
  (`UserWidget.AddToViewport` _output_get 0))

(event `self.ReceiveTick`
  (params (DeltaSeconds :type "Float (single-precision)"))
  (bind _currentactor (`self.CurrentActor`))
  (bind _camera (`self.Camera`))
  (bind _returnvalue (`SceneComponent.K2_GetComponentLocation` _camera))
  ;[1 1 1] Line Trace
  (bind _outhit (`KismetSystemLibrary.LineTraceSingle` :`Start` _returnvalue :`End` (+ _returnvalue (* (`SceneComponent.GetForwardVector` _camera) 1000.0)) :`TraceChannel` "TraceTypeQuery1" :`DrawDebugType` "ForOneFrame"))
  (if (`GameplayStatics.BreakHitResult` _outhit)
    (set `self.LineTracingObject?` true)
    (if (`KismetSystemLibrary.DoesImplementInterface` (`.HitActor` (`GameplayStatics.BreakHitResult` _outhit)) "/Game/Blueprints/iInteract.iInteract_C")
      (set `self.ObjectHasInterface` true)
      (if (!= (`.HitActor` (`GameplayStatics.BreakHitResult` _outhit)) (`self.CurrentActor`))
        (set `self.CurrentActor` (`.HitActor` (`GameplayStatics.BreakHitResult` _outhit))) ; Set CurrentActor to overlapped object
      )
      (else
        (set `self.ObjectHasInterface` false)
        (`/Engine/EditorBlueprintResources/StandardMacros.IsValid` _currentactor :!label _label ; is currentactor valid
          (:`Is Valid`
            (message `/Game/Blueprints/iInteract.NonInteractable` _currentactor))
          (:`Is Not Valid`
            (set `self.CurrentActor` null) ; if not, set current actor to null
          ))))
    (else
      (set `self.LineTracingObject?` false)
      (goto _label))))

(event `InputAxis|Strafe`
  (params (AxisValue :type "Float (single-precision)"))
  ;[1 1 1] Controls
  (`PawnMovementComponent.AddInputVector` (`self.CharacterMovement`) (* (`self.GetActorRightVector`) AxisValue) false))

(event `InputAxis|Walk`
  (params (AxisValue :type "Float (single-precision)"))
  ;[1 1 1] Controls
  (`PawnMovementComponent.AddInputVector` (`self.CharacterMovement`) (* (`self.GetActorForwardVector`) AxisValue) false))

(event `InputAxis|Turn`
  (params (AxisValue :type "Float (single-precision)"))
  ;[1 1 1] Controls
  (`self.AddControllerYawInput` AxisValue))

(event `InputAxis|Up/Down`
  (params (AxisValue :type "Float (single-precision)"))
  ;[1 1 1] Controls
  (`self.AddControllerPitchInput` AxisValue))

(event `InputAction|Interact`
  (params (Key :type "Key Structure"))
  (bind _currentactor (`self.CurrentActor`))
  ;[1 1 1] Controls
  (:`Pressed`
    (if (and (== (`self.LineTracingObject?`) true) (== (`self.ObjectHasInterface`) true))
      (`/Engine/EditorBlueprintResources/StandardMacros.IsValid` _currentactor
        (:`Is Valid`
          (message `/Game/Blueprints/iInteract.Interactable` _currentactor))))))

(event `InputAction|Pickup`
  (params (Key :type "Key Structure"))
  ;[1 1 1] Controls
  (:`Pressed`
    (`KismetSystemLibrary.PrintString` "space bar pressed")
    (`/Game/UI/InventoryWidget.SpaceBar` (`self.InventoryWidget`))))

(fn `AddItemMC`
  (params (`New Item` :type "Texture2D Object Reference") (HashCode :type String))
  (`/Game/UI/InventoryWidget.AddItemToInv` (`self.InventoryWidget`) `New Item` HashCode))

(fn `UserConstructionScript`)