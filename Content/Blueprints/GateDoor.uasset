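; GateDoor is a gate actor that opens and closes along its local Z axis through the OpenDoor and CloseDoor events.
; Each event plays the same bike-chain sound at the actor's location and starts its own timeline, Open or Close.
; Timeline updates add the track value as a local offset to the Gate component without sweep, so movement accumulates per tick and total travel depends on frame rate.
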(event `OpenDoor`
  ;[1 1 1] Door Opens
  (`GameplayStatics.PlaySoundAtLocation` "/Game/Blueprints/AudioStuffs/AudioStorage/484470__inspectorj__bike-chain-spinning-fast-02-01.484470__inspectorj__bike-chain-spinning-fast-02-01" (`self.K2_GetActorLocation`) (struct) 1.0 1.0 0.0 null null null)
  (bind (_direction _upward) (`Timeline|Open`)
    (:`Update`
      (`SceneComponent.K2_AddLocalOffset` (`self.Gate`) (`KismetMathLibrary.MakeVector` 0.0 0.0 _upward) false false))))

(event `CloseDoor`
  ;[1 1 1] Door Closes
  (`GameplayStatics.PlaySoundAtLocation` "/Game/Blueprints/AudioStuffs/AudioStorage/484470__inspectorj__bike-chain-spinning-fast-02-01.484470__inspectorj__bike-chain-spinning-fast-02-01" (`self.K2_GetActorLocation`) (struct) 1.0 1.0 0.0 null null null)
  (bind (_direction _newtrack_0) (`Timeline|Close`)
    (:`Update`
      (`SceneComponent.K2_AddLocalOffset` (`self.Gate`) (`KismetMathLibrary.MakeVector` 0.0 0.0 _newtrack_0) false false))))

(fn `UserConstructionScript`)