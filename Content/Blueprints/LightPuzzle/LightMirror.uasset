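; LightMirror is a rotatable mirror for a light puzzle that lights up when it receives light from another active mirror.
; Interacting rotates Mirrortop by a set amount, and mirrors flagged active at BeginPlay start lit with one light source.
; StaticMesh overlaps with active mirrors raise or lower a source count, which switches the spotlight on, or off at zero.
; The point light is hidden whenever the state updates, and debug prints trace changes.
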(event `self.ReceiveBeginPlay`
  ;[1 1 1] Setup
  (if (`self.IsActive`)
    (set `self.Source` 1)
    (`SceneComponent.SetVisibility` (`self.SpotLight`) true false)
    (`SceneComponent.SetVisibility` (`self.PointLight`) false false)
    (`KismetSystemLibrary.PrintString` "StartingMirrorGood")))

(event `/Game/Blueprints/iInteract.Interactable`
  ;[1 1 1] Rotate
  (`SceneComponent.K2_AddLocalRotation` (`self.Mirrortop`) (`self.Rotation amount`) true false))

(event `self.StaticMesh.OnComponentBeginOverlap`
  (params (OverlappedComponent :type "PrimitiveComponent Object Reference") (OtherActor :type "Actor Object Reference") (OtherComp :type "PrimitiveComponent Object Reference") (OtherBodyIndex :type Integer) (bFromSweep :type Boolean) (SweepResult :type "HitResult Structure (by ref)"))
  ;[1 1 1] On hitting Mirrors
  (bind _aslight_mirror (cast `/Game/Blueprints/LightPuzzle/LightMirror` OtherActor))
  (if (`/Game/Blueprints/LightPuzzle/LightMirror.IsActive` _aslight_mirror)
    (set `self.IsActive` true)
    (`SceneComponent.SetVisibility` (`self.SpotLight`) true false)
    (`SceneComponent.SetVisibility` (`self.PointLight`) false false)
    (`KismetSystemLibrary.PrintString` "Active Mirror Hit!")
    (set `self.Source` (+ (`self.Source`) 1))))

(event `self.StaticMesh.OnComponentEndOverlap`
  (params (OverlappedComponent :type "PrimitiveComponent Object Reference") (OtherActor :type "Actor Object Reference") (OtherComp :type "PrimitiveComponent Object Reference") (OtherBodyIndex :type Integer))
  ;[1 1 1] On moving away from Mirrors
  (bind _aslight_mirror (cast `/Game/Blueprints/LightPuzzle/LightMirror` OtherActor))
  (if (`/Game/Blueprints/LightPuzzle/LightMirror.IsActive` _aslight_mirror)
    (set `self.Source` (- (`self.Source`) 1))
    (`KismetSystemLibrary.PrintString` "Mirror Moved Away")
    (if (not (>= (`self.Source`) 1))
      (`KismetSystemLibrary.PrintString` "No more light Source")
      (`SceneComponent.SetVisibility` (`self.SpotLight`) false false)
      (`SceneComponent.SetVisibility` (`self.PointLight`) false false)
      (set `self.IsActive` false))))

(fn `UserConstructionScript`)