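; LightGoal is the target actor of the light mirror puzzle, marking it solved when an active mirror reaches it.
; Its Goal component's begin overlap casts the other actor to LightMirror and calls PuzzleSolve if that mirror is active.
; PuzzleSolve sets the Solved flag, zeroes RotationAmount on every LightMirror in the level to freeze them, and prints debug messages.
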(event `self.Goal.OnComponentBeginOverlap`
  (params (OverlappedComponent :type "PrimitiveComponent Object Reference") (OtherActor :type "Actor Object Reference") (OtherComp :type "PrimitiveComponent Object Reference") (OtherBodyIndex :type Integer) (bFromSweep :type Boolean) (SweepResult :type "HitResult Structure (by ref)"))
  (bind _aslight_mirror (cast `/Game/Blueprints/LightPuzzle/LightMirror` OtherActor))
  (if (`/Game/Blueprints/LightPuzzle/LightMirror.IsActive` _aslight_mirror)
    (`self.PuzzleSolve`)))

(fn `PuzzleSolve`
  (`KismetSystemLibrary.PrintString` "PuzzleSolved")
  (set `self.Solved?` true)
  (bind _outactors (`GameplayStatics.GetAllActorsOfClass` "/Game/Blueprints/LightPuzzle/LightMirror.LightMirror_C"))
  (for _array_element _outactors
    (set `/Game/Blueprints/LightPuzzle/LightMirror.Rotation amount` (struct) _array_element)
    (`KismetSystemLibrary.PrintString` "Mirrors Immobile, Puzzle Done" true true (struct :`R` 1.0 :`G` 0.08466 :`A` 1.0))))

(fn `UserConstructionScript`)