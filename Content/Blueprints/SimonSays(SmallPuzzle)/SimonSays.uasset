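; Simon Says mini-puzzle actor with four colored lights, each paired with an overlap box the main character steps into to answer.
; BeginPlay rolls one random color sequence, and the first box touched starts the game.
; A PlayColors/EnableLight delay loop shows a longer prefix in each of three stages, with input locked during playback.
; Mistakes replay the current stage; finishing calls PuzzleIsDone, currently an empty stub.
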(event `self.ReceiveBeginPlay`
  ;[1 1 1] On BeginPlay, Setting up the puzzle
  (`self.CreateSequence`)
  (`SceneComponent.SetVisibility` (`self.LightB`) false false)
  (`SceneComponent.SetVisibility` (`self.LightG`) false false)
  (`SceneComponent.SetVisibility` (`self.LightR`) false false)
  (`SceneComponent.SetVisibility` (`self.LightY`) false false))

(event `Puzzle Is Done`
  ;[1 1 1] Puzzle Completed
)

(event `self.BoxR.OnComponentBeginOverlap`
  (params (OverlappedComponent :type "PrimitiveComponent Object Reference") (OtherActor :type "Actor Object Reference") (OtherComp :type "PrimitiveComponent Object Reference") (OtherBodyIndex :type Integer) (bFromSweep :type Boolean) (SweepResult :type "HitResult Structure (by ref)"))
  (bind _lightr (`self.LightR`))
  ;[1 1 1] General Overlap Start
  (cast `/Game/Blueprints/MainCharacter` OtherActor)
  (if (`self.CanPress`)
    (`SceneComponent.SetVisibility` _lightr true false)
    (`KismetSystemLibrary.Delay` 0.6)
    (`SceneComponent.SetVisibility` _lightr false false)
    (if (`self.Active`)
      (bind _output_get (set `self.PlayerColor` 1))
      (`GameplayStatics.PlaySoundAtLocation` "/Game/Blueprints/AudioStuffs/AudioStorage/543048__clusman__as-ab-al-computer-noise-6-16bit.543048__clusman__as-ab-al-computer-noise-6-16bit" (`self.K2_GetActorLocation`) (struct) 1.0 1.0 0.0 null null null)
      (`self.SimonCheckThis` _output_get)
      (else
        (set `self.Active` true)
        (`self.StartTheFun` :!label _label)))))

(event `self.BoxB.OnComponentBeginOverlap`
  (params (OverlappedComponent :type "PrimitiveComponent Object Reference") (OtherActor :type "Actor Object Reference") (OtherComp :type "PrimitiveComponent Object Reference") (OtherBodyIndex :type Integer) (bFromSweep :type Boolean) (SweepResult :type "HitResult Structure (by ref)"))
  (bind _lightb (`self.LightB`))
  ;[1 1 1] General Overlap Start
  (cast `/Game/Blueprints/MainCharacter` OtherActor)
  (if (`self.CanPress`)
    (`SceneComponent.SetVisibility` _lightb true false)
    (`KismetSystemLibrary.Delay` 0.6)
    (`SceneComponent.SetVisibility` _lightb false false)
    (if (`self.Active`)
      (bind _output_get (set `self.PlayerColor` 2))
      (`GameplayStatics.PlaySoundAtLocation` "/Game/Blueprints/AudioStuffs/AudioStorage/543048__clusman__as-ab-al-computer-noise-6-16bit.543048__clusman__as-ab-al-computer-noise-6-16bit" (`self.K2_GetActorLocation`) (struct) 1.0 1.0 0.0 null null null)
      (`self.SimonCheckThis` _output_get)
      (else
        (set `self.Active` true)
        (goto _label)))))

(event `self.BoxG.OnComponentBeginOverlap`
  (params (OverlappedComponent :type "PrimitiveComponent Object Reference") (OtherActor :type "Actor Object Reference") (OtherComp :type "PrimitiveComponent Object Reference") (OtherBodyIndex :type Integer) (bFromSweep :type Boolean) (SweepResult :type "HitResult Structure (by ref)"))
  (bind _lightg (`self.LightG`))
  ;[1 1 1] General Overlap Start
  (cast `/Game/Blueprints/MainCharacter` OtherActor)
  (if (`self.CanPress`)
    (`SceneComponent.SetVisibility` _lightg true false)
    (`KismetSystemLibrary.Delay` 0.6)
    (`SceneComponent.SetVisibility` _lightg false false)
    (if (`self.Active`)
      (bind _output_get (set `self.PlayerColor` 3))
      (`GameplayStatics.PlaySoundAtLocation` "/Game/Blueprints/AudioStuffs/AudioStorage/543048__clusman__as-ab-al-computer-noise-6-16bit.543048__clusman__as-ab-al-computer-noise-6-16bit" (`self.K2_GetActorLocation`) (struct) 1.0 1.0 0.0 null null null)
      (`self.SimonCheckThis` _output_get)
      (else
        (set `self.Active` true)
        (goto _label)))))

(event `self.BoxY.OnComponentBeginOverlap`
  (params (OverlappedComponent :type "PrimitiveComponent Object Reference") (OtherActor :type "Actor Object Reference") (OtherComp :type "PrimitiveComponent Object Reference") (OtherBodyIndex :type Integer) (bFromSweep :type Boolean) (SweepResult :type "HitResult Structure (by ref)"))
  (bind _lighty (`self.LightY`))
  ;[1 1 1] General Overlap Start
  (cast `/Game/Blueprints/MainCharacter` OtherActor)
  (if (`self.CanPress`)
    (`SceneComponent.SetVisibility` _lighty true false)
    (`KismetSystemLibrary.Delay` 0.6)
    (`SceneComponent.SetVisibility` _lighty false false)
    (if (`self.Active`)
      (bind _output_get (set `self.PlayerColor` 4))
      (`GameplayStatics.PlaySoundAtLocation` "/Game/Blueprints/AudioStuffs/AudioStorage/543048__clusman__as-ab-al-computer-noise-6-16bit.543048__clusman__as-ab-al-computer-noise-6-16bit" (`self.K2_GetActorLocation`) (struct) 1.0 1.0 0.0 null null null)
      (`self.SimonCheckThis` _output_get)
      (else
        (set `self.Active` true)
        (goto _label)))))

(event `StartTheFun`
  ;[1 1 1] Begin here
  (`self.FlashLights`)
  ;[1 1 1] Setup
  (`KismetSystemLibrary.PrintString` "SimonSaysStart")
  (set `self.CanPress` false)
  (set `self.Part1` true)
  (`KismetSystemLibrary.Delay` 2.0)
  (`self.PlayPattern`))

(event `FlashLights`
  (bind _lightb (`self.LightB`))
  (bind _lightg (`self.LightG`))
  (bind _lighty (`self.LightY`))
  (bind _lightr (`self.LightR`))
  ;[1 1 1] Flash Lights
  (`SceneComponent.SetVisibility` _lightr true false)
  (`SceneComponent.SetVisibility` _lightb true false)
  (`SceneComponent.SetVisibility` _lightg true false)
  (`SceneComponent.SetVisibility` _lighty true false)
  (`KismetSystemLibrary.Delay` 0.6)
  (`SceneComponent.SetVisibility` _lightr false false)
  (`SceneComponent.SetVisibility` _lightb false false)
  (`SceneComponent.SetVisibility` _lightg false false)
  (`SceneComponent.SetVisibility` _lighty false false))

(event `PlayColors`
  ;[1 1 1] Color Loop
  (if (< (`self.CurrentIndex`) (`self.SequenceLength`))
    (`self.EnableLight` (select `int` (`|GetArrayItem` (`self.Sequence`) (`self.CurrentIndex`)) :`0` null :`1` (`self.LightR`) :`2` (`self.LightB`) :`3` (`self.LightG`) :`4` (`self.LightY`)))
    (`/Engine/EditorBlueprintResources/StandardMacros.IncrementInt` (`self.CurrentIndex`))
    (else
      (set `self.CanPress` true))))

(event `PlayPattern`
  ;[1 1 1] Entry
  (if (`self.Part1`)
    (set `self.SequenceLength` 4)
    (set `self.CanPress` false)
    (`self.PlayColors`)
    (elif (`self.Part2`)
      (set `self.SequenceLength` 5)
      (set `self.CanPress` false)
      (`self.PlayColors`)
      (elif (`self.Part3`)
        (set `self.SequenceLength` 6)
        (set `self.CanPress` false)
        (`self.PlayColors`)
        (elif (`self.Completed`)
          (set `self.CanPress` false)
          (`self.Puzzle Is Done`)
          (else
            (`KismetSystemLibrary.PrintString` "ErrorPlayPattern")))))))

(event `EnableLight`
  (params (Light :type "PointLightComponent Object Reference"))
  ;[1 1 1] Lights Lighting up (Will add sound here)
  (`GameplayStatics.PlaySoundAtLocation` "/Game/Blueprints/AudioStuffs/AudioStorage/543048__clusman__as-ab-al-computer-noise-6-16bit.543048__clusman__as-ab-al-computer-noise-6-16bit" (`self.K2_GetActorLocation`) (struct) 1.0 1.0 0.0 null null null)
  (`SceneComponent.SetVisibility` Light true false)
  (`KismetSystemLibrary.Delay` 0.6)
  (`SceneComponent.SetVisibility` Light false false)
  (`KismetSystemLibrary.Delay` 0.3)
  (`self.PlayColors`))

(event `SimonCheckThis`
  (params (RBGY :type Integer))
  (bind _playerindex (`self.PlayerIndex`))
  (bind _playerindex_2 (`self.PlayerIndex`))
  ;[1 1 1] PlayerChecking
  (`KismetArrayLibrary.Array_Insert` (`self.PlayerInput`) RBGY (`self.PlayerIndex`))
  (if (== (`|GetArrayItem` (`self.Sequence`) _playerindex_2) (`|GetArrayItem` (`self.PlayerInput`) _playerindex_2))
    (`KismetSystemLibrary.PrintString` "Correct")
    (if (< _playerindex (- (`self.SequenceLength`) 1))
      (`/Engine/EditorBlueprintResources/StandardMacros.IncrementInt` _playerindex
        (:`  `
          (`KismetSystemLibrary.PrintString` (`KismetStringLibrary.Conv_IntToString` _playerindex))))
      (elif (`self.Part1`)
        (set `self.Part1` false)
        (set `self.Part2` true)
        (`KismetSystemLibrary.PrintString` "Part 1 Done")
        (set `self.CurrentIndex` 0 :!label _label_2)
        (set `self.PlayerIndex` 0)
        (`KismetSystemLibrary.Delay` 1.0)
        (`self.PlayPattern`)
        (elif (`self.Part2`)
          (set `self.Part2` false)
          (set `self.Part3` true)
          (`KismetSystemLibrary.PrintString` "Part 2 Done")
          (goto _label_2)
          (elif (`self.Part3`)
            (set `self.Part3` false)
            (set `self.Completed` true)
            (`KismetSystemLibrary.PrintString` "Part 3 Done")
            (goto _label_2)))))
    (else
      (`KismetSystemLibrary.PrintString` "WRONG")
      (set `self.PlayerIndex` 0)
      (set `self.PlayerColor` 0)
      (set `self.CurrentIndex` 0)
      (`KismetArrayLibrary.Array_Clear` (`self.PlayerInput`))
      (`self.FlashLights`)
      (`KismetSystemLibrary.Delay` 1.0)
      (`self.PlayPattern`))))

(fn `CreateSequence`
  (bind _output_get (set `self.Sequence` (`|MakeArray` (`KismetMathLibrary.RandomIntegerInRange` 1 4) (`KismetMathLibrary.RandomIntegerInRange` 1 4) (`KismetMathLibrary.RandomIntegerInRange` 1 4) (`KismetMathLibrary.RandomIntegerInRange` 1 4) (`KismetMathLibrary.RandomIntegerInRange` 1 4) (`KismetMathLibrary.RandomIntegerInRange` 1 4))))
  (for _array_element _output_get
    (`KismetSystemLibrary.PrintString` (`KismetStringLibrary.Conv_IntToString` _array_element)))
  (`KismetSystemLibrary.PrintString` "SimonSays Randomly Setup"))

(fn `UserConstructionScript`)