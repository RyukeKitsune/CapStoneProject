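; Interactive door actor that the player swings open and shut with the Action input or a first-finger touch while inside its trigger box.
; Trigger overlap events open or close a Gate and enable or disable input for the first player controller.
; The Closed flag selects playing or reversing a timeline that drives the door mesh's relative yaw, and a FlipFlop on timeline completion toggles that flag.
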(event `InputAction|Action`
  (params (Key :type "Key Structure"))
  ;[1 1 1] Input
  (:`Pressed`
    (`/Engine/EditorBlueprintResources/StandardMacros.Gate` true :!label _label
      (:`Exit`
        ;[1 1 1] Closed?
        (if (`self.Closed?`)
          ;[1 1 1] Door Rotation
          (bind (_direction _doorrotation) (`Timeline|Timeline_0` :!label _label_2)
            (:`Update`
              (`SceneComponent.K2_SetRelativeRotation` (`self.Door_01A`) (`KismetMathLibrary.MakeRotator` 0.0 0.0 _doorrotation) false false))
            (:`Finished`
              (`/Engine/EditorBlueprintResources/StandardMacros.FlipFlop`
                (:`A`
                  (set `self.Closed?` false))
                (:`B`
                  (set `self.Closed?` true)))))
          (else
            (goto _label_2 :!via `Reverse`)))))))

(event `InputTouch`
  (params (Location :type "Vector Structure") (FingerIndex :type "ETouchIndex Enum"))
  ;[1 1 1] Input
  (:`Pressed`
    (if (`|EnumEquality` FingerIndex "Touch1")
      (goto _label))))

(event `self.TriggerBox.OnComponentBeginOverlap`
  (params (OverlappedComponent :type "PrimitiveComponent Object Reference") (OtherActor :type "Actor Object Reference") (OtherComp :type "PrimitiveComponent Object Reference") (OtherBodyIndex :type Integer) (bFromSweep :type Boolean) (SweepResult :type "HitResult Structure (by ref)"))
  ;[1 1 1] Input
  (`self.EnableInput` (`GameplayStatics.GetPlayerController` 0))
  (goto _label :!via `Open`))

(event `self.TriggerBox.OnComponentEndOverlap`
  (params (OverlappedComponent :type "PrimitiveComponent Object Reference") (OtherActor :type "Actor Object Reference") (OtherComp :type "PrimitiveComponent Object Reference") (OtherBodyIndex :type Integer))
  ;[1 1 1] Input
  (`self.DisableInput` (`GameplayStatics.GetPlayerController` 0))
  (goto _label :!via `Close`))

(fn `UserConstructionScript`)