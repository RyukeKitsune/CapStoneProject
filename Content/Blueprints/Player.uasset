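; First-person style player character with movement, mouse-look style axes and line-trace interaction with actors implementing IInteract.
; Tick traces a short ray forward from the camera and caches the interactable it hits as CurrentActor.
; Interact sends InteractableMessage to that actor, while looking elsewhere sends it NonInteractableMessage every tick.
; A valid CurrentActor is never cleared, so Interact still reaches it after the view moves away.
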(event `self.ReceiveTick`
  (params (DeltaSeconds :type "Float (single-precision)"))
  (bind _currentactor (`self.CurrentActor`))
  (bind _camera (`self.Camera`))
  (bind _returnvalue (`SceneComponent.K2_GetComponentLocation` _camera))
  (bind _outhit (`KismetSystemLibrary.LineTraceSingle` :`Start` _returnvalue :`End` (+ _returnvalue (* (`SceneComponent.GetForwardVector` _camera) 1000.0)) :`TraceChannel` "TraceTypeQuery1" :`DrawDebugType` "ForOneFrame"))
  (if (`GameplayStatics.BreakHitResult` _outhit)
    (if (`KismetSystemLibrary.DoesImplementInterface` (`.HitActor` (`GameplayStatics.BreakHitResult` _outhit)) "/Game/Blueprints/iInteract.iInteract_C")
      (if (!= (`.HitActor` (`GameplayStatics.BreakHitResult` _outhit)) (`self.CurrentActor`))
        (set `self.CurrentActor` (`.HitActor` (`GameplayStatics.BreakHitResult` _outhit))))
      (else
        (`/Engine/EditorBlueprintResources/StandardMacros.IsValid` _currentactor :!label _label
          (:`Is Valid`
            (message `/Game/Blueprints/iInteract.NonInteractable` _currentactor))
          (:`Is Not Valid`
            (set `self.CurrentActor` null)))))
    (else
      (goto _label))))

(event `InputAxis|Strafe`
  (params (AxisValue :type "Float (single-precision)"))
  ;[1 1 1] Controls
  (`PawnMovementComponent.AddInputVector` (`self.CharacterMovement`) (* (`self.GetActorRightVector`) AxisValue) false))

(event `InputAxis|Walk`
  (params (AxisValue :type "Float (single-precision)"))
  ;[1 1 1] Controls
  (`PawnMovementComponent.AddInputVector` (`self.CharacterMovement`) (* (`self.GetActorForwardVector`) AxisValue) false))

(event `InputAxis|Turn`
  (params (AxisValue :type "Float (single-precision)"))
  ;[1 1 1] Controls
  (`self.AddControllerYawInput` AxisValue))

(event `InputAxis|Up/Down`
  (params (AxisValue :type "Float (single-precision)"))
  ;[1 1 1] Controls
  (`self.AddControllerPitchInput` AxisValue))

(event `InputAction|Interact`
  (params (Key :type "Key Structure"))
  (bind _currentactor (`self.CurrentActor`))
  ;[1 1 1] Controls
  (:`Pressed`
    (`/Engine/EditorBlueprintResources/StandardMacros.IsValid` _currentactor
      (:`Is Valid`
        (message `/Game/Blueprints/iInteract.Interactable` _currentactor)))))

(fn `UserConstructionScript`)