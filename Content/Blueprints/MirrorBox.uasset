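; MirrorBox is an interactable Blueprint that gives the player a mirror item the first time it is used.
; BeginPlay gathers the top-level InventoryWidget instances.
; Interactable uses the first widget to call FoundObject and AddItemToInv with the mirror data from InventoryStruct.
; An Interacted flag blocks repeat pickups, and debug prints trace each step.
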(event `self.ReceiveBeginPlay`
  (bind _foundwidgets (`WidgetBlueprintLibrary.GetAllWidgetsOfClass` "/Game/UI/InventoryWidget.InventoryWidget_C")))

(event `/Game/Blueprints/iInteract.Interactable`
  (bind (_inventorystruct_key _inventorystruct_statuette _inventorystruct_mirror _inventorystruct_mirrorhc) (break `/Game/Blueprints/InventoryStruct` (`self.InventoryStruct`)))
  (if (not (`self.Interacted?`))
    (`KismetSystemLibrary.PrintString` "Before found object, interacted" true true (struct :`G` 0.66 :`B` 1.0 :`A` 1.0) 20.0)
    (bind _output (`|GetArrayItem` (stale `self.ReceiveBeginPlay` _foundwidgets)))
    (`/Game/UI/InventoryWidget.FoundObject` _output _inventorystruct_mirror)
    (`KismetSystemLibrary.PrintString` "found object called" true true (struct :`G` 0.66 :`B` 1.0 :`A` 1.0) 20.0)
    (set `self.Interacted?` true)
    (`KismetSystemLibrary.PrintString` "interacted set to true" true true (struct :`G` 0.66 :`B` 1.0 :`A` 1.0) 20.0)
    (`/Game/UI/InventoryWidget.AddItemToInv` _output _inventorystruct_mirror _inventorystruct_mirrorhc)
    (`KismetSystemLibrary.PrintString` "add item to inv called" true true (struct :`G` 0.66 :`B` 1.0 :`A` 1.0) 20.0)))

(fn `UserConstructionScript`)